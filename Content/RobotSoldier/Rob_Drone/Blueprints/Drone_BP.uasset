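; Drone actor that circles the world origin on Tick, always turning to face a fixed point above it.
; It hops between waypoints on a fixed-radius ring, each a random angular step onward at a randomized height.
; Speed grows by a per-frame multiplier until halfway to the waypoint, then decays toward a minimum, easing each hop without timelines or physics.
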(event `self.ReceiveTick`
  (params (DeltaSeconds :type "Float (single-precision)"))
  (bind _returnvalue (`KismetMathLibrary.RandomFloatInRange` 35.0 45.0))
  (bind _returnvalue_2 (`self.K2_GetActorLocation`))
  (bind _topos (`self.ToPos`))
  (bind _speed (`self.Speed`))
  (bind _returnvalue_3 (`KismetMathLibrary.Vector_Distance` _topos _returnvalue_2))
  (bind _returnvalue_4 (- _topos _returnvalue_2))
  (bind _returnvalue_5 (+ (`self.Angle`) _returnvalue))
  ;[1 1 1] Move Drone around
  (`self.K2_SetActorRotation` (`KismetMathLibrary.FindLookAtRotation` _returnvalue_2 (`KismetMathLibrary.MakeVector` 0.0 0.0 170.0)))
  (if (< (`KismetMathLibrary.VSize` _returnvalue_4) 2.0)
    (set `self.ToPos` (`KismetMathLibrary.MakeVector` (* (`KismetMathLibrary.DegCos` _returnvalue_5) 333.0) (* (`KismetMathLibrary.DegSin` _returnvalue_5) 333.0) (* _returnvalue 6.0)))
    (set `self.Angle` _returnvalue_5)
    (set `self.Dist` _returnvalue_3)
    (set `self.Speed` 22.0)
    (else
      (`self.K2_SetActorLocation` (+ (* (* (`KismetMathLibrary.Normal` _returnvalue_4) DeltaSeconds) (`self.Speed`)) _returnvalue_2))
      (if (< (/ (`self.Dist`) 2.0) _returnvalue_3)
        (set `self.Speed` (* _speed 1.01))
        (elif (> _speed 22.0)
          (set `self.Speed` (* _speed 0.99)))))))

(fn `UserConstructionScript`)